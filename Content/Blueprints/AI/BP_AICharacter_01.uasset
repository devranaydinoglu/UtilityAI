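; BP_AICharacter_01 is an AI character whose Patrol and ChasePlayer events act as example movement tasks for a utility AI task manager.
; It caches its BP_AIController_01 on BeginPlay.
; Each task deactivates the controller's UtilityTaskManager, runs AI MoveTo toward a random nearby navigable point or the player, then reactivates the manager and puts that task on cooldown, whether the move succeeds or fails.
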(event `self.ReceiveBeginPlay`
  ;[1 1 1] Set reference to character's ai controller
  (bind _asbp_aicontroller_01 (cast `/Game/Blueprints/AI/BP_AIController_01` (`self.GetController`)))
  (set `self.AIController` _asbp_aicontroller_01))

(event `Patrol`
  ;[1 1 1] Example MoveTo task
  (`UtilityTaskManagerComponent.DeactivateUTM` (`/Game/Blueprints/AI/BP_AIController_01.UtilityTaskManager` (`self.AIController`)))
  (`|AIMoveTo` self (`NavigationSystemV1.K2_GetRandomLocationInNavigableRadius` (`self.K2_GetActorLocation`) 800.0 null null) null
    (:`OnSuccess`
      _)
    (:`OnFail`
      _))
  (`UtilityTaskManagerComponent.ActivateUTM` (`/Game/Blueprints/AI/BP_AIController_01.UtilityTaskManager` (`self.AIController`)))
  (`UtilityTaskManagerComponent.SetCooldown` (`/Game/Blueprints/AI/BP_AIController_01.UtilityTaskManager` (`self.AIController`)) "/Game/Blueprints/AI/UtilityTasks/UT_Patrol_AI_01.UT_Patrol_AI_01_C" 3.0 false false))

(event `ChasePlayer`
  (bind _returnvalue (`GameplayStatics.GetPlayerCharacter` 0))
  (`UtilityTaskManagerComponent.DeactivateUTM` (`/Game/Blueprints/AI/BP_AIController_01.UtilityTaskManager` (`self.AIController`)))
  (`|AIMoveTo` self (`self.K2_GetActorLocation` _returnvalue) _returnvalue
    (:`OnSuccess`
      _)
    (:`OnFail`
      _))
  (`UtilityTaskManagerComponent.ActivateUTM` (`/Game/Blueprints/AI/BP_AIController_01.UtilityTaskManager` (`self.AIController`)))
  (`UtilityTaskManagerComponent.SetCooldown` (`/Game/Blueprints/AI/BP_AIController_01.UtilityTaskManager` (`self.AIController`)) "/Game/Blueprints/AI/UtilityTasks/UT_ChasePlayer_AI_01.UT_ChasePlayer_AI_01_C" 3.0 false false))

(fn `UserConstructionScript`)