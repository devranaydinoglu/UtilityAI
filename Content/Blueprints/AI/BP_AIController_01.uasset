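; AI controller that drives an agent through a UtilityTaskManager component and tracks whether it senses the player.
; It initializes the manager on BeginPlay and prints the active task's name every tick for debugging.
; AIPerception target updates set IsPlayerSensed from the stimulus for BP_ThirdPersonCharacter, and clear it when any other actor triggers an update.
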(event `self.ReceiveBeginPlay`
  ;[1 1 1] Initialize UTM component
  (`UtilityTaskManagerComponent.Initialize` (`self.UtilityTaskManager`)))

(event `self.ReceiveTick`
  (params (DeltaSeconds :type "Float (single-precision)"))
  (`KismetSystemLibrary.PrintString` (`KismetSystemLibrary.GetDisplayName` (`UtilityTaskManagerComponent.ActiveTask` (`self.UtilityTaskManager`)))))

(event `self.AIPerception.OnTargetPerceptionUpdated`
  (params (Actor :type "Actor Object Reference") (Stimulus :type "AIStimulus Structure"))
  ;[1 1 1] On target perception updated
  (cast `/Game/Blueprints/BP_ThirdPersonCharacter` Actor
    (:`then`
      (set `self.bIsPlayerSensed` (`.bSuccessfullySensed` (break `AIStimulus` Stimulus))))
    (:`CastFailed`
      (set `self.bIsPlayerSensed` false))))

(fn `UserConstructionScript`)